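; BP_Water is a configurable water surface actor that turns its exposed variables into a tuned water material.
; The construction script first calls InitialWaterCreation, which creates a dynamic material instance on WaterSurface and sets its X/Y scale.
; It then pushes settings for colour, opacity, ripples, Gerstner waves, shoreline, caustics, tessellation and normal maps into that instance.
; Boolean toggles reach the material as float scalar parameters.
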(fn ConstructionScript
  (bind _water_material (Variables|Default|GetWater%20Material))
  (|InitialWaterCreation)
  (Rendering|Material|SetScalarParameterValue _water_material "Fade Distance Opacity" (Variables|Shoreline|GetOpacity) :!class /Script/Engine.MaterialInstanceDynamic)
  (Rendering|Material|SetScalarParameterValue _water_material "Small Wave Speed" (Variables|NormalMapWaves|GetSmall%20Wave%20Speed) :!class /Script/Engine.MaterialInstanceDynamic)
  (Rendering|Material|SetScalarParameterValue _water_material "Large Wave Speed" (Variables|NormalMapWaves|GetLarge%20Wave%20Speed) :!class /Script/Engine.MaterialInstanceDynamic)
  (Rendering|Material|SetScalarParameterValue _water_material "LargeRipples" (Variables|NormalMapWaves|GetLarge%20Ripple%20Scale) :!class /Script/Engine.MaterialInstanceDynamic)
  (Rendering|Material|SetScalarParameterValue _water_material "DistanceFromShore" (Variables|Shoreline|GetShore%20Falloff) :!class /Script/Engine.MaterialInstanceDynamic)
  (Rendering|Material|SetScalarParameterValue _water_material "Debug MDF" (Math|Conversions|ToFloat(Boolean) (Variables|Debug|GetDebug%20MDF)) :!class /Script/Engine.MaterialInstanceDynamic)
  (Rendering|Material|SetScalarParameterValue _water_material "Gerstner Waves" (Math|Conversions|ToFloat(Boolean) (Variables|GerstnerWaves|GetGerstner%20Waves)) :!class /Script/Engine.MaterialInstanceDynamic)
  (Rendering|Material|SetScalarParameterValue _water_material "Shore Mask" (Math|Conversions|ToFloat(Boolean) (Variables|Shoreline|GetShore%20Mask)) :!class /Script/Engine.MaterialInstanceDynamic)
  (Rendering|Material|SetVectorParameterValue _water_material "Dark_Colour" (Variables|Colour|GetDark%20Water%20Colour) :!class /Script/Engine.MaterialInstanceDynamic)
  (Rendering|Material|SetVectorParameterValue _water_material "Light_Color" (Variables|Colour|GetLight%20Water%20Color) :!class /Script/Engine.MaterialInstanceDynamic)
  (Rendering|Material|SetScalarParameterValue _water_material "Wavelength" (Variables|GerstnerWaves|GetWavelength) :!class /Script/Engine.MaterialInstanceDynamic)
  (Rendering|Material|SetScalarParameterValue _water_material "Amplitude" (Variables|GerstnerWaves|GetAmplitude) :!class /Script/Engine.MaterialInstanceDynamic)
  (Rendering|Material|SetScalarParameterValue _water_material "Number of Waves" (Variables|GerstnerWaves|GetNumber%20of%20Waves) :!class /Script/Engine.MaterialInstanceDynamic)
  (Rendering|Material|SetScalarParameterValue _water_material "Steepness" (Variables|GerstnerWaves|GetSteepness) :!class /Script/Engine.MaterialInstanceDynamic)
  (Rendering|Material|SetScalarParameterValue _water_material "Speed" (Variables|GerstnerWaves|GetSpeed) :!class /Script/Engine.MaterialInstanceDynamic)
  (Rendering|Material|SetVectorParameterValue _water_material "Wave Direction 1" (Variables|GerstnerWaves|GetWave%20Direction%201) :!class /Script/Engine.MaterialInstanceDynamic)
  (Rendering|Material|SetVectorParameterValue _water_material "Wave Direction 2" (Variables|GerstnerWaves|GetWave%20Direction%202) :!class /Script/Engine.MaterialInstanceDynamic)
  (Rendering|Material|SetVectorParameterValue _water_material "Wave Direction 3" (Variables|GerstnerWaves|GetWave%20Direction%203) :!class /Script/Engine.MaterialInstanceDynamic)
  (Rendering|Material|SetVectorParameterValue _water_material "Wave Direction 4" (Variables|GerstnerWaves|GetWave%20Direction%204) :!class /Script/Engine.MaterialInstanceDynamic)
  (Rendering|Material|SetScalarParameterValue _water_material "Tesselation" (Variables|Default|GetTesselation%20Multiplier) :!class /Script/Engine.MaterialInstanceDynamic)
  (Rendering|Material|SetScalarParameterValue _water_material "Caustic Brightness" (Variables|Caustics|GetCaustic%20Brightness) :!class /Script/Engine.MaterialInstanceDynamic)
  (Rendering|Material|SetScalarParameterValue _water_material "Caustic Fade Distance" (Variables|Caustics|GetCaustics%20Depth) :!class /Script/Engine.MaterialInstanceDynamic)
  (Rendering|Material|SetScalarParameterValue _water_material "RGB Split Speed" (Variables|Caustics|GetRGB%20Split%20Speed) :!class /Script/Engine.MaterialInstanceDynamic)
  (Rendering|Material|SetScalarParameterValue _water_material "Caustic Size" (Variables|Caustics|GetCaustics%20Tiling) :!class /Script/Engine.MaterialInstanceDynamic)
  (Rendering|Material|SetScalarParameterValue _water_material "Water Caustics" (Math|Conversions|ToFloat(Boolean) (Variables|Caustics|GetWater%20Caustics)) :!class /Script/Engine.MaterialInstanceDynamic)
  (Rendering|Material|SetScalarParameterValue _water_material "SkyAtmosphere" (Math|Conversions|ToFloat(Boolean) (Variables|Caustics|GetSkyAtmosphere)) :!class /Script/Engine.MaterialInstanceDynamic)
  (Rendering|Material|SetVectorParameterValue _water_material "CausticsColour" (Variables|Caustics|GetCausticsColour) :!class /Script/Engine.MaterialInstanceDynamic)
  (Rendering|Material|SetTextureParameterValue _water_material "SmallWaves" (Variables|NormalMapWaves|GetSmall%20Waves%20Normal))
  (Rendering|Material|SetTextureParameterValue _water_material "DistanceWaves" (Variables|NormalMapWaves|GetDistance%20Waves%20Normal))
  (Rendering|Material|SetTextureParameterValue _water_material "LargeWaves" (Variables|NormalMapWaves|GetLarge%20Waves%20Normal)))